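; BP_ElevatorTrigger is a box trigger that sends its referenced Elevator up or down, per ToGoUp, while a BP_ThirdPersonCharacter overlaps it.
; Overlap events track the player, and Tick repeats the GoUp or GoDown call whenever the activation cooldown has elapsed.
; With StickToElevator set, it stores its platform-local offset at BeginPlay and moves itself with the platform every Tick.
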(event `self.ReceiveBeginPlay`
  (set `self.OffSetToElevatorifSticking` (0.0 0.0 0.0))
  (if (`self.bStickToElevator`)
    (`/Engine/EditorBlueprintResources/StandardMacros.IsValid` (`self.Elevator`)
      (:`Is Valid`
        (set `self.OffSetToElevatorifSticking` (`KismetMathLibrary.InverseTransformLocation` (`/Game/ElevatorSystem/Elevator/BP_Elevator.GetPlatformTransform` (`self.Elevator`)) (`self.K2_GetActorLocation`)))))))

(event `self.ReceiveTick`
  (params (DeltaSeconds :type "Float (single-precision)"))
  (bind _elevator (`self.Elevator`))
  (`|ExecutionSequence`
    (:`then_0`
      (set `self.timeElapsedSinceLastActivation` (+ DeltaSeconds (`self.timeElapsedSinceLastActivation`)))
      (if (`self.bStickToElevator`)
        (`/Engine/EditorBlueprintResources/StandardMacros.IsValid` (`self.Elevator`)
          (:`Is Valid`
            (`self.K2_SetActorLocation` (`KismetMathLibrary.TransformLocation` (`/Game/ElevatorSystem/Elevator/BP_Elevator.GetPlatformTransform` (`self.Elevator`)) (`self.OffSetToElevatorifSticking`)) true true)))))
    (:`then_1`
      (if (`self.bPlayerOverlapping`)
        (if (> (`self.timeElapsedSinceLastActivation`) (`self.ActivationCooldown`))
          (`|ExecutionSequence`
            (:`then_0`
              (if (`self.bToGoUp`)
                (`/Game/ElevatorSystem/Elevator/BP_Elevator.GoUp` _elevator)
                (else
                  (`/Game/ElevatorSystem/Elevator/BP_Elevator.GoDown` _elevator))))
            (:`then_1`
              (set `self.timeElapsedSinceLastActivation` 0.0))))))))

(event `self.Box.OnComponentBeginOverlap`
  (params (OverlappedComponent :type "PrimitiveComponent Object Reference") (OtherActor :type "Actor Object Reference") (OtherComp :type "PrimitiveComponent Object Reference") (OtherBodyIndex :type Integer) (bFromSweep :type Boolean) (SweepResult :type "HitResult Structure (by ref)"))
  (bind _asbp_third_person_character (cast `/Game/ElevatorSystem/Character/BP_ThirdPersonCharacter` OtherActor))
  (set `self.thirdPersonCharacter` _asbp_third_person_character)
  (set `self.bPlayerOverlapping` true))

(event `self.Box.OnComponentEndOverlap`
  (params (OverlappedComponent :type "PrimitiveComponent Object Reference") (OtherActor :type "Actor Object Reference") (OtherComp :type "PrimitiveComponent Object Reference") (OtherBodyIndex :type Integer))
  (cast `/Game/ElevatorSystem/Character/BP_ThirdPersonCharacter` OtherActor)
  (set `self.bPlayerOverlapping` false)
  (set `self.thirdPersonCharacter` null))

(fn `UserConstructionScript`)