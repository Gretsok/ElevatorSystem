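; Elevator actor whose platform mesh moves and rotates between floors defined by an array of anchor actors.
; GoUp and GoDown step a clamped floor index and convert that anchor's transform to actor-local targets, with index zero being the actor's origin.
; Tick lerps the mesh toward the target using a smoothing value, snapping when within one step.
; GetPlatformTransform exposes the mesh's world transform.
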(event `self.ReceiveTick`
  (params (DeltaSeconds :type "Float (single-precision)"))
  (bind _returnvalue (- (`KismetMathLibrary.VLerp` (`SceneComponent.RelativeLocation` (`self.StaticMesh`)) (`self.CurrentTargetPosition`) (* DeltaSeconds (`self.MovementSmoothValue`))) (`SceneComponent.RelativeLocation` (`self.StaticMesh`))))
  (if (< (`KismetMathLibrary.Vector_Distance` (`self.CurrentTargetPosition`) (`SceneComponent.RelativeLocation` (`self.StaticMesh`))) (`KismetMathLibrary.VSize` _returnvalue))
    (`SceneComponent.K2_SetRelativeRotation` (`self.StaticMesh`) (`self.CurrentTargetRotator`) false false)
    (`SceneComponent.K2_SetRelativeLocation` (`self.StaticMesh`) (`self.CurrentTargetPosition`) false false)
    (else
      (`SceneComponent.K2_SetRelativeLocation` (`self.StaticMesh`) (+ (`SceneComponent.RelativeLocation` (`self.StaticMesh`)) _returnvalue) false false)
      (`SceneComponent.K2_SetRelativeRotation` (`self.StaticMesh`) (`KismetMathLibrary.RLerp` (`SceneComponent.RelativeRotation` (`self.StaticMesh`)) (`self.CurrentTargetRotator`) (* DeltaSeconds (`self.MovementSmoothValue`))) false false))))

(fn `GetPlatformTransform`
  (returns (PlatformTransform :type "Transform Structure"))
  (return (`SceneComponent.K2_GetComponentToWorld` (`self.StaticMesh`))))

(fn `GoDown`
  (bind _returnvalue (`self.GetTransform`))
  (bind _output_get (set `self.CurrentFloorIndex` (`KismetMathLibrary.Clamp` (+ (`self.CurrentFloorIndex`) -1) 0 (`KismetArrayLibrary.Array_Length` (`self.FloorAnchors`)))))
  (`KismetSystemLibrary.PrintString` (`KismetStringLibrary.Conv_IntToString` _output_get))
  (if (> _output_get 0)
    (bind _output (`|GetArrayItem` (`self.FloorAnchors`) (- _output_get 1)))
    (set `self.CurrentTargetPosition` (`KismetMathLibrary.InverseTransformLocation` _returnvalue (`self.K2_GetActorLocation` _output)))
    (set `self.CurrentTargetRotator` (`KismetMathLibrary.InverseTransformRotation` _returnvalue (`self.K2_GetActorRotation` _output)))
    (else
      (set `self.CurrentTargetPosition` (0.0 0.0 0.0))
      (set `self.CurrentTargetRotator` (struct)))))

(fn `GoUp`
  (bind _returnvalue (`self.GetTransform`))
  (bind _output_get (set `self.CurrentFloorIndex` (`KismetMathLibrary.Clamp` (+ (`self.CurrentFloorIndex`) 1) 0 (`KismetArrayLibrary.Array_Length` (`self.FloorAnchors`)))))
  (if (> _output_get 0)
    (bind _returnvalue_2 (- _output_get 1))
    (`KismetSystemLibrary.PrintString` (`KismetStringLibrary.Conv_IntToString` _returnvalue_2))
    (bind _output (`|GetArrayItem` (`self.FloorAnchors`) _returnvalue_2))
    (set `self.CurrentTargetPosition` (`KismetMathLibrary.InverseTransformLocation` _returnvalue (`self.K2_GetActorLocation` _output)))
    (set `self.CurrentTargetRotator` (`KismetMathLibrary.InverseTransformRotation` _returnvalue (`self.K2_GetActorRotation` _output)))
    (else
      (`KismetSystemLibrary.PrintText` "ok")
      (set `self.CurrentTargetPosition` (0.0 0.0 0.0))
      (set `self.CurrentTargetRotator` (struct)))))

(fn `UserConstructionScript`)